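; BP_Chunk is a terrain chunk actor with a ground plane sized to one chunk.
; Its construction script derives the chunk's side length from the block count and block size in DA_TerrainSettings class defaults.
; It scales GroundPlane in X and Y by that length over 100, then offsets it by half the length so the actor origin sits at a corner.
; BeginPlay is empty.
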(event EventBeginPlay)

(fn ConstructionScript
  (bind (_chunkblocks _blocksize) (Utilities|GetClassDefaults "/Game/OurContent/Terrain/DA_TerrainSettings.DA_TerrainSettings_C"))
  (bind _groundplane (Variables|Default|GetGroundPlane))
  (bind _returnvalue (* _chunkblocks _blocksize))
  (bind _returnvalue_2 (Math|Conversions|ToFloat(Integer) _returnvalue))
  (bind _returnvalue_3 (/ _returnvalue_2 100))
  (bind _returnvalue_4 (/ _returnvalue_2 2))
  (bind _returnvalue_5 (Math|Conversions|ToFloat(Integer) _returnvalue_3))
  (bind _returnvalue_6 (Math|Conversions|ToFloat(Integer) _returnvalue_4))
  (Transformation|SetRelativeScale3D _groundplane (Math|Vector|MakeVector _returnvalue_5 _returnvalue_5 1.0))
  (Transformation|SetRelativeLocation _groundplane (Math|Vector|MakeVector _returnvalue_6 _returnvalue_6 0.0) false false))