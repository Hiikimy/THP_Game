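; Base combat character for player and enemies, handling health, melee attacks, hit flash and death.
; A looping timer and key events derive dead, attacking, moving or idle state, broadcasting changes and disabling movement and capsule collision on death.
; Attacks alter walk speed and lock movement-based rotation until a timer scaled by attack speed ends them.
; Hits use a forward sphere trace, letting players damage any pawn but AI only the player.
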(event Custom|StateTick
  (if (not (Utilities|Enum|Equal(Enum) (Variables|Default|GetCharacterState) "NewEnumerator3"))
    (CallFunction|RefreshState)))

(event EventBeginPlay
  (Variables|Default|SetHealth (Variables|Default|GetMaxHealth))
  (Variables|/Script/Engine.CharacterMovementComponent|SetMaxWalkSpeed (Variables|Character|GetCharacterMovement) (Variables|Default|GetWalkSpeed))
  (Utilities|Time|SetTimerbyEvent (delegate Custom|StateTick) 0.1 true true))

(event Game|Damage|EventAnyDamage
  (params (Damage :type Float%20%28single-precision%29) (DamageType :type Damage%20Type%20Object%20Reference) (InstigatedBy :type Controller%20Object%20Reference) (DamageCauser :type Actor%20Object%20Reference))
  (CallFunction|RecieveDamage Damage)
  (Rendering|Material|SetOverlayMaterial (Variables|Character|GetMesh) "/Game/OurContent/Characters/Materials/M_HitFlash.M_HitFlash" false 0 :!class /Script/Engine.MeshComponent)
  (Utilities|FlowControl|RetriggerableDelay (Variables|Default|GetHitFlashDuration))
  (Rendering|Material|SetOverlayMaterial (Variables|Character|GetMesh) 0 false 0 :!class /Script/Engine.MeshComponent))

(fn ConstructionScript)

(fn RefreshState
  (if (<= (Variables|Default|GetHealth) 0.0)
    (LocalVariables|SetNewState "NewEnumerator3")
    (elif (Variables|Default|GetisAttacking)
      (LocalVariables|SetNewState "NewEnumerator1")
      (elif (Utilities|Operators|NotEqual(!=) :A (Variables|/Script/Engine.MovementComponent|GetVelocity (Variables|Character|GetCharacterMovement)) :ErrorTolerance 3.0)
        (LocalVariables|SetNewState "NewEnumerator4")
        (else
          (LocalVariables|SetNewState "NewEnumerator0")))))
  (if (Utilities|Enum|NotEqual(Enum) (LocalVariables|GetNewState) (Variables|Default|GetCharacterState))
    (LocalVariables|SetOldState (Variables|Default|GetCharacterState))
    (Variables|Default|SetCharacterState (LocalVariables|GetNewState))
    (Default|CallOnStateChange (LocalVariables|GetNewState) (LocalVariables|GetOldState))
    (if (Utilities|Enum|Equal(Enum) (LocalVariables|GetNewState) "NewEnumerator3")
      (CallFunction|Die))))

(fn SetHP
  (params (NewValue :type Float%20%28double-precision%29))
  (bind _maxhealth (Variables|Default|GetMaxHealth))
  (bind _output_get (Variables|Default|SetHealth (Math|Float|Clamp(Float) NewValue 0.0 _maxhealth)))
  (Default|CallOnHPChanged _output_get _maxhealth)
  (CallFunction|RefreshState)
  (Development|PrintString (Utilities|String|Append (Utilities|String|Append (Utilities|GetObjectName (Game|GetPlayerController 0)) "'s HP changed to: ") (Utilities|String|ToString(Float) (Variables|Default|GetHealth))) false false))

(fn RecieveDamage
  (params (Damage :type Float%20%28double-precision%29))
  (if (Utilities|Enum|NotEqual(Enum) (Variables|Default|GetCharacterState) "NewEnumerator3")
    (CallFunction|SetHP (- (Variables|Default|GetHealth) Damage))))

(fn StartAttack
  (bind _charactermovement (Variables|Character|GetCharacterMovement))
  (if (or (Utilities|Enum|Equal(Enum) (Variables|Default|GetCharacterState) "NewEnumerator3") (Variables|Default|GetisAttacking))
    (return false)
    (else
      (Variables|Default|SetisAttacking true)
      (CallFunction|RefreshState)
      (Utilities|Time|SetTimerbyFunctionName 0 "EndAttack" (/ 1.0 (Math|Float|Max(Float) (Variables|Default|GetAttackSpeed) 0.01)))
      (Variables|/Script/Engine.CharacterMovementComponent|SetMaxWalkSpeed _charactermovement (* (Variables|Default|GetWalkSpeed) (Variables|Default|GetAttackMoveMult)))
      (Variables|/Script/Engine.CharacterMovementComponent|SetbOrientRotationToMovement _charactermovement false)
      (return true))))

(fn EndAttack
  (bind _charactermovement (Variables|Character|GetCharacterMovement))
  (Variables|Default|SetisAttacking false)
  (Animation|Montage|MontageStop (Components|SkeletalMesh|GetAnimInstance (Variables|Character|GetMesh)) 0.0 0)
  (Variables|/Script/Engine.CharacterMovementComponent|SetMaxWalkSpeed _charactermovement (Variables|Default|GetWalkSpeed))
  (Variables|/Script/Engine.CharacterMovementComponent|SetbOrientRotationToMovement _charactermovement true)
  (CallFunction|RefreshState))

(fn Die
  (Variables|Default|SetisAttacking false)
  (Default|CallOnDeath)
  (Pawn|Components|CharacterMovement|DisableMovement (Variables|Character|GetCharacterMovement))
  (Collision|SetCollisionEnabled (Variables|Collision|GetCapsuleComponent) "NoCollision"))

(fn DoAttackHit
  (bind _returnvalue (Transformation|GetActorLocation))
  (bind _outhits (Collision|MultiSphereTraceForObjects _returnvalue (+ _returnvalue (* (Transformation|GetActorForwardVector) (Variables|Default|GetAttackRange))) (Variables|Default|GetAttackRadius) (Utilities|Array|MakeArray "ObjectTypeQuery3") false (Utilities|Array|MakeArray self) "None" true "(R=1.000000,G=0.000000,B=0.000000,A=1.000000)" "(R=0.000000,G=1.000000,B=0.000000,A=1.000000)" (Variables|Default|GetAttackSpeed)))
  (for _array_element _outhits
    (LocalVariables|SetHitActor (.HitActor (Collision|BreakHitResult _array_element)))
    (if (and (not (Utilities|Array|ContainsItem (LocalVariables|GetHitActors) (LocalVariables|GetHitActor))) (or (== (LocalVariables|GetHitActor) (Game|Player|GetPlayerPawn 0)) (Pawn|IsPlayerControlled)))
      (Utilities|Array|Add (LocalVariables|GetHitActors) (LocalVariables|GetHitActor))
      (Game|Damage|ApplyDamage (LocalVariables|GetHitActor) (Variables|Default|GetAttackDamage) (Pawn|GetController) self))))