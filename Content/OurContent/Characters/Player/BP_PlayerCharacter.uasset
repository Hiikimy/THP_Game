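; Player character Blueprint with cursor-driven controls, adding Enhanced Input movement and melee attack on top of its parent class.
; WASD moves along axes yawed 45 degrees, while click-to-move paths to the cursor hit via SimpleMoveToLocation; one character state blocks both.
; Attacking turns the character toward the cursor, and if StartAttack succeeds, stops movement, plays a sword montage and calls DoAttackHit after a delay, both scaled by AttackSpeed.
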(event Input|EnhancedActionEvents|EnhancedInputActionIA_Move
  (params (ActionValue :type Vector%202D%20Structure) (ElapsedSeconds :type Float%20%28double-precision%29) (TriggeredSeconds :type Float%20%28double-precision%29) (InputAction :type Input%20Action%20Object%20Reference :default "/Game/OurContent/Characters/Player/IA_Move.IA_Move"))
  (bind _returnvalue (Math|Rotator|MakeRotator 0.0 0.0 45.0))
  (bind (_x _y) (Math|Vector2D|BreakVector2D ActionValue))
  ;[0.15 0.15 0.15 0.5] WASD Movement
  (:Triggered
    (if (Utilities|Enum|NotEqual(Enum) (Variables|Default|GetCharacterState) "NewEnumerator3")
      (Pawn|Input|AddMovementInput (Math|Vector|GetForwardVector _returnvalue) _y false)
      (Pawn|Input|AddMovementInput (Math|Vector|GetRightVector _returnvalue) _x false)))
  (:Started
    (Components|Movement|StopMovementImmediately (Variables|Character|GetCharacterMovement))))

(event Input|EnhancedActionEvents|EnhancedInputActionIA_ClickMove
  (params (ActionValue :type Boolean) (ElapsedSeconds :type Float%20%28double-precision%29) (TriggeredSeconds :type Float%20%28double-precision%29) (InputAction :type Input%20Action%20Object%20Reference :default "/Game/OurContent/Characters/Player/IA_ClickMove.IA_ClickMove"))
  (bind _returnvalue (Game|GetPlayerController 0))
  (bind _hitresult (Game|Player|GetHitResultUnderCursorbyChannel _returnvalue "TraceTypeQuery1" false))
  (bind _location (Collision|BreakHitResult _hitresult))
  ;[0.15 0.15 0.15 0.5] Click Movement (When dist > 50)
  (if (Utilities|Enum|NotEqual(Enum) (Variables|Default|GetCharacterState) "NewEnumerator3")
    (if (> (Math|Vector|VectorLength (- _location (Transformation|GetActorLocation _returnvalue))) 5e+01)
      (AI|Navigation|SimpleMovetoLocation _returnvalue _location))))

(event Input|EnhancedActionEvents|EnhancedInputActionIA_Attack
  (params (ActionValue :type Boolean) (ElapsedSeconds :type Float%20%28double-precision%29) (TriggeredSeconds :type Float%20%28double-precision%29) (InputAction :type Input%20Action%20Object%20Reference :default "/Game/OurContent/Characters/Player/IA_Attack.IA_Attack"))
  (bind _returnvalue (Game|GetPlayerController 0))
  (bind (_hitresult _returnvalue_2) (Game|Player|GetHitResultUnderCursorbyChannel _returnvalue "TraceTypeQuery1" false))
  ;[0.15 0.15 0.15 0.5] Starting attacking sequence
  (if _returnvalue_2
    (Transformation|SetActorRotation (Math|Rotator|MakeRotator 0.0 0.0 (.Yaw (Math|Rotator|BreakRotator (Math|Rotator|FindLookatRotation (Transformation|GetActorLocation) (.Location (Collision|BreakHitResult _hitresult)))))))
    (bind _success (CallFunction|StartAttack))
    (if _success
      (AI|Navigation|StopMovement (Pawn|GetController))
      (Animation|PlayAnimMontage "/Game/OurContent/Characters/Models/FBX/WarriorCharacterArmature_Sword_Attack_Montage.WarriorCharacterArmature_Sword_Attack_Montage" (* 0.8333 (Variables|Default|GetAttackSpeed)) "None")
      (Utilities|FlowControl|Delay (/ 0.8 (Variables|Default|GetAttackSpeed)))
      (CallFunction|DoAttackHit))))

(event EventBeginPlay
  (bind _returnvalue (Game|GetPlayerController 0))
  (|CallParentFunction)
  (Variables|/Script/Engine.PlayerController|SetbShowMouseCursor _returnvalue true)
  (Input|AddMappingContext (PlayerController|LocalPlayerSubsystems|GetEnhancedInputLocalPlayerSubsystem _returnvalue) "/Game/OurContent/Characters/Player/IMC_Player.IMC_Player" 0 "(bIgnoreAllPressedKeysUntilRelease=True,bForceImmediately=False,bNotifyUserSettings=False)"))

(fn ConstructionScript)