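; Melee enemy Blueprint that extends a parent enemy class with a montage-driven attack and range-checked damage to the player.
; StartAttack plays the attack montage only when the parent's StartAttack succeeds, and returns that result.
; ApplyMeleeHit, not called within this Blueprint, applies damage to player pawn 0 if it is within attack range, using a distance check instead of collision.
; The event graph adds no logic of its own.
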(event EventBeginPlay
  (|CallParentFunction) ; This node is disabled and will not be called.\nDrag off pins to build functionality.
)

(event Collision|EventActorBeginOverlap
  (params (OtherActor :type Actor%20Object%20Reference)))

(event EventTick
  (params (DeltaSeconds :type Float%20%28single-precision%29)))

(fn ConstructionScript
  (|CallParentFunction))

(fn StartAttack
  (bind _success (|CallParentFunction))
  (if _success
    (Animation|PlayAnimMontage (Variables|Default|GetAttackMontage) 1.0 "None")
    (return _success)
    (else
      (return false))))

(fn ApplyMeleeHit
  (bind _returnvalue (Game|Player|GetPlayerPawn 0))
  (Utilities|IsValid _returnvalue
    (:Is%20Valid
      (if (<= (Transformation|GetDistanceTo _returnvalue) (Variables|Default|GetAttackRange))
        (Game|Damage|ApplyDamage (Game|Player|GetPlayerPawn 0) (Variables|Default|GetAttackDamage) 0 self "/Script/Engine.DamageType")))))