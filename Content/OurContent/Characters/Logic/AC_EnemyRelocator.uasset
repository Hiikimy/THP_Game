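; Actor component for BP_EnemyDirector that leashes active enemies to the player by teleporting stragglers to offscreen points.
; A looping timer, pausable through SetEnabled, checks horizontal distance against LeashRadius and caps relocation attempts with MaxPerCheck.
; Each relocation asks the director for an offscreen point using the enemy-to-player direction, lifts it by capsule half-height, then stops the controller's movement.
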(event Custom|OnLeashTimer
  (CallFunction|CheckLeash))

(event Custom|SetEnabled
  (params (Enabled :type Boolean))
  (bind _leashtimer (Variables|Default|GetLeashTimer))
  (if Enabled
    (Utilities|Time|UnpauseTimerbyHandle _leashtimer)
    (else
      (Utilities|Time|PauseTimerbyHandle _leashtimer))))

(event EventBeginPlay
  (bind _asbp_enemy_director (Utilities|Casting|CastToBP_EnemyDirector (Components|GetOwner)))
  (Variables|Default|SetDirector _asbp_enemy_director)
  (bind _returnvalue (Utilities|Time|SetTimerbyEvent (delegate Custom|OnLeashTimer) (Variables|Default|GetCheckInterval) true))
  (Variables|Default|SetLeashTimer _returnvalue))

(fn RelocateEnemy
  (params (Enemy :type BP%20Enemy%20Object%20Reference) (PlayerLoc :type Vector))
  (bind (_location _found) (Default|GetOffscreenPoint (Variables|Default|GetDirector) (- PlayerLoc (Transformation|GetActorLocation Enemy))))
  (if _found
    (Transformation|SetActorLocation Enemy (+ _location (Math|Vector|MakeVector 0.0 0.0 (Components|Capsule|GetScaledCapsuleHalfHeight (Variables|/Script/Engine.Character|GetCapsuleComponent Enemy)))) false true)
    (AI|Navigation|StopMovement (Pawn|GetController Enemy))
    (return true)
    (else
      (return false))))

(fn CheckLeash
  (bind _returnvalue (Game|GetPlayerCharacter 0))
  (for _array_element (Variables|/Game/OurContent/Characters/Logic/BP_EnemyDirector.BP_EnemyDirector_C|GetActiveEnemies (Variables|Default|GetDirector))
    (Utilities|IsValid _array_element
      (:Is%20Valid
        (if (and (> (Transformation|GetHorizontalDistanceTo _array_element _returnvalue) (Variables|Default|GetLeashRadius)) (< (LocalVariables|GetCount) (Variables|Default|GetMaxPerCheck)))
          (CallFunction|RelocateEnemy _array_element (Transformation|GetActorLocation _returnvalue))
          (LocalVariables|SetCount (+ (LocalVariables|GetCount) 1)))))))