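; Enemy spawner component for the BP_EnemyDirector actor that spawns enemies by time-based waves.
; A looping timer, pausable via SetEnabled, picks the DT_Waves row whose minute window contains the time since BeginPlay.
; Each enemy entry spawns up to its per-tick count, capped by MaxAlive minus the director's alive count for that class.
; Spawns use director-supplied offscreen points in random directions, raised by a Z offset.
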(event Custom|OnSpawnTimer
  (CallFunction|SpawnTick))

(event Custom|SetEnabled
  (params (Enabled :type Boolean))
  (bind _spawntimer (Variables|Default|GetSpawnTimer))
  (if Enabled
    (Utilities|Time|UnpauseTimerbyHandle _spawntimer)
    (else
      (Utilities|Time|PauseTimerbyHandle _spawntimer))))

(event EventBeginPlay
  (bind _asbp_enemy_director (Utilities|Casting|CastToBP_EnemyDirector (Components|GetOwner)))
  (Variables|Default|SetDirector _asbp_enemy_director)
  (Variables|Default|SetRunStartTime (Utilities|Time|GetGameTimeinSeconds))
  (bind _returnvalue (Utilities|Time|SetTimerbyEvent (delegate Custom|OnSpawnTimer) (Variables|Default|GetSpawnInterval) true))
  (Variables|Default|SetSpawnTimer _returnvalue))

(fn GetActiveWave
  (LocalVariables|SetElapsedMin (/ (- (Utilities|Time|GetGameTimeinSeconds) (Variables|Default|GetRunStartTime)) 6e+01))
  (bind _outrownames (DataTable|GetDataTableRowNames "/Game/OurContent/Characters/Logic/DT_Waves.DT_Waves"))
  (for _array_element _outrownames
    (bind _returnvalue (Utilities|GetDataTableRow "/Game/OurContent/Characters/Logic/DT_Waves.DT_Waves" _array_element)
      (:then
        (if (and (<= (.StartMin (Utilities|Struct|BreakS_Wave _returnvalue)) (LocalVariables|GetElapsedMin)) (< (LocalVariables|GetElapsedMin) (.EndMin (Utilities|Struct|BreakS_Wave _returnvalue))))
          (return true _returnvalue)))))
  (return false ""))

(fn SpawnOne
  (params (EnemyClass :type BP%20Enemy%20Class%20Reference))
  (bind (_location _found) (Default|GetOffscreenPoint (Variables|Default|GetDirector) (Math|Vector|RotateVectorAroundAxis "1.000000,0.000000,0.000000" (Math|Random|RandomFloatinRange 0.0 3.6e+02) "0.000000,0.000000,1.000000")))
  (if (and _found (Utilities|IsValidClass EnemyClass))
    (Game|SpawnActorfromClass EnemyClass (Math|Transform|MakeTransform (+ _location (Math|Vector|MakeVector 0.0 0.0 (Variables|Default|GetSpawnZOffset)))) "AdjustIfPossibleButAlwaysSpawn" "SelectDefaultAtRuntime" 0 2e+01 0)))

(fn SpawnTick
  (bind (_found _wave) (CallFunction|GetActiveWave))
  (if _found
    (for _array_element (.Enemies (Utilities|Struct|BreakS_Wave _wave))
      (LocalVariables|SetToSpawn (Math|Integer|Min(Integer) (.SpawnPerTick (Utilities|Struct|BreakS_WaveEnemy _array_element)) (- (.MaxAlive (Utilities|Struct|BreakS_WaveEnemy _array_element)) (.Value (Utilities|Map|Find (Variables|/Game/OurContent/Characters/Logic/BP_EnemyDirector.BP_EnemyDirector_C|GetAliveByClass (Variables|Default|GetDirector)) (.EnemyClass (Utilities|Struct|BreakS_WaveEnemy _array_element)))))))
      (for _index (range 1 (LocalVariables|GetToSpawn))
        (CallFunction|SpawnOne (.EnemyClass (Utilities|Struct|BreakS_WaveEnemy _array_element)))))))