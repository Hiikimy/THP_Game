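; Enemy director that tracks active enemies and finds navigable spawn points around the player.
; Register and unregister calls maintain a unique active-enemy list and per-class alive counts, printing both.
; GetOffscreenPoint retries jittered directions at randomized radii, projecting each onto the navmesh; "offscreen" relies on distance alone, with no visibility check.
; Nothing spawns here, and the debug sphere timer is disconnected.
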(event Custom|DebugPoint
  ;[0.15 0.15 0.15 0.5] Debug (F8)
  (bind (_location _found) (CallFunction|GetOffscreenPoint (Math|Vector|RotateVectorAroundAxis "1.000000,0.000000,0.000000" (Math|Random|RandomFloatinRange 0.0 3.6e+02) "0.000000,0.000000,1.000000")))
  (if _found
    (Rendering|Debug|DrawDebugSphere _location 5e+01 12 "(R=1.000000,G=0.000000,B=0.000000,A=1.000000)" 3.0)
    (Development|PrintString (Utilities|String|ToString(Vector) _location))))

(event EventBeginPlay)

(fn ConstructionScript)

(fn RegisterEnemy
  (params (Enemy :type BP%20Enemy%20Object%20Reference))
  (bind _returnvalue (Utilities|GetClass Enemy))
  (bind _activeenemies (Variables|Default|GetActiveEnemies))
  (bind _alivebyclass (Variables|Default|GetAliveByClass))
  (bind _value (Utilities|Map|Find _alivebyclass _returnvalue))
  (bind _returnvalue_2 (Utilities|Array|AddUnique _activeenemies Enemy))
  (if (!= _returnvalue_2 -1)
    (Utilities|Map|Add _alivebyclass _returnvalue (+ _value 1))
    (Development|PrintString (Utilities|String|Append "Registered. Alive: " (Utilities|String|ToString(Integer) (Utilities|Array|Length _activeenemies)) " | " (Utilities|GetClassDisplayName _returnvalue) ": " (Utilities|String|ToString(Integer) _value)))))

(fn UnregisterEnemy
  (params (Enemy :type BP%20Enemy%20Object%20Reference))
  (bind _returnvalue (Utilities|GetClass Enemy))
  (bind _activeenemies (Variables|Default|GetActiveEnemies))
  (bind _alivebyclass (Variables|Default|GetAliveByClass))
  (bind _value (Utilities|Map|Find _alivebyclass _returnvalue))
  (bind _returnvalue_2 (Utilities|Array|RemoveItem _activeenemies Enemy))
  (if _returnvalue_2
    (Utilities|Map|Add _alivebyclass _returnvalue (- _value 1))
    (Development|PrintString (Utilities|String|Append "Unregistered. Alive: " (Utilities|String|ToString(Integer) (Utilities|Array|Length _activeenemies)) " | " (Utilities|GetClassDisplayName _returnvalue) ": " (Utilities|String|ToString(Integer) _value)))))

(fn GetOffscreenPoint
  (params (Direction :type Vector))
  (bind _returnvalue (Game|GetPlayerCharacter 0))
  (bind _jitterdeg (Variables|Default|GetJitterDeg))
  (bind _spawnradius (Variables|Default|GetSpawnRadius))
  (Utilities|IsValid _returnvalue
    (:Is%20Valid
      (LocalVariables|SetPlayerLoc (Transformation|GetActorLocation _returnvalue))
      (LocalVariables|SetDir2D (Math|Vector|Normalize (* Direction "1.000000,1.000000,0.000000")))
      (for _index (range 1 (Variables|Default|GetMaxTries))
        (bind _output_get (LocalVariables|SetCandidate (+ (LocalVariables|GetPlayerLoc) (* (Math|Vector|RotateVectorAroundAxis (LocalVariables|GetDir2D) (Math|Random|RandomFloatinRange (* _jitterdeg -1.0) _jitterdeg) "0.000000,0.000000,1.000000") (Math|Random|RandomFloatinRange _spawnradius (+ _spawnradius (Variables|Default|GetSpawnRadiusVariance)))))))
        (if (.ReturnValue (AI|Navigation|ProjectPointtoNavigation _output_get 0 0 (Variables|Default|GetNavQueryExtent)))
          (return (.ProjectedLocation (AI|Navigation|ProjectPointtoNavigation _output_get 0 0 (Variables|Default|GetNavQueryExtent))) true)
          (else
            (Development|PrintString "NO POINT")))))
    (:Is%20Not%20Valid
      _))
  (return "0, 0, 0" false))