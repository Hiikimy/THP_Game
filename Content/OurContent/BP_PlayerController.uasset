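; BP_PlayerController is a player controller that sets up the player's HUD when it possesses a character.
; On possess, it casts the pawn to BP_Character and stops for any other pawn type.
; It creates WBP_PlayerHUD and adds it to the viewport only if none exists, then calls the HUD's Init with the possessed character on every successful possession.
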(event EventPossess
  (params (PossessedPawn :type Pawn%20Object%20Reference))
  (bind _asbp_character (Utilities|Casting|CastToBP_Character PossessedPawn))
  (if (not (Utilities|IsValid (Variables|Default|GetHUD)))
    (bind _returnvalue (UserInterface|CreateWidget "/Game/OurContent/Characters/UI/WBP_PlayerHUD.WBP_PlayerHUD_C" self))
    (bind _output_get (Variables|Default|SetHUD _returnvalue))
    (UserInterface|Viewport|AddtoViewport _output_get 0))
  (Default|Init (Variables|Default|GetHUD) _asbp_character))

(fn ConstructionScript)