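; Terrain generator that streams BP_Chunk actors in a square grid around the player, sized from DA_TerrainSettings defaults.
; A looping timer queues missing chunks within RenderDistance and destroys loaded ones beyond it plus a one-chunk margin.
; A faster timer pops one queued coordinate per tick and spawns that chunk, spreading out spawn cost.
; Loaded chunks are tracked in a map keyed by chunk coordinate.
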(event Custom|BuildTimer
  ;[0.15 0.15 0.15 0.5] Spawn vždy max 1 chunku za 1 tick
  (bind (_found _chunk) (CallFunction|GetfromQueue))
  (if _found
    (CallFunction|SpawnChunk _chunk)))

(event Custom|UpdateTimer
  (CallFunction|UpdateChunks))

(event EventBeginPlay
  (Utilities|Time|SetTimerbyEvent (delegate Custom|UpdateTimer) 0.5 true true)
  ;[0.15 0.15 0.15 0.5] Hned po načtení
  (CallFunction|UpdateChunks)
  ;[0.15 0.15 0.15 0.5] Spawn vždy max 1 chunku za 1 tick
  (Utilities|Time|SetTimerbyEvent (delegate Custom|BuildTimer) 0.1 true))

(fn ConstructionScript)

(fn SpawnChunk
  (params (Chunk :type S%20Chunk%20Structure))
  (bind (_x _y) (Utilities|Struct|BreakS_Chunk Chunk))
  (bind (_chunkblocks _blocksize) (Utilities|GetClassDefaults "/Game/Terrain/DA_TerrainSettings.DA_TerrainSettings_C"))
  (bind _returnvalue (* _chunkblocks _blocksize))
  (bind _returnvalue_2 (Game|SpawnActorfromClass "/Game/Terrain/BP_Chunk.BP_Chunk_C" (Math|Conversions|ToTransform(Vector) (Math|Vector|MakeVector (Math|Conversions|ToFloat(Integer) (* _x _returnvalue)) (Math|Conversions|ToFloat(Integer) (* _y _returnvalue)) 0.0)) "AlwaysSpawn" "MultiplyWithRoot" 0 Chunk 0))
  (Utilities|Map|Add (Variables|Default|GetLoadedChunks) Chunk _returnvalue_2))

(fn UpdateChunks
  (bind _renderdistance (Variables|Default|GetRenderDistance))
  (bind _spawnqueue (Variables|Default|GetSpawnQueue))
  (bind _playerchunk (CallFunction|GetPlayerChunk))
  (for _index (range (- (.X (Utilities|Struct|BreakS_Chunk _playerchunk)) _renderdistance) (+ (.X (Utilities|Struct|BreakS_Chunk _playerchunk)) _renderdistance))
    (for _index_2 (range (- (.Y (Utilities|Struct|BreakS_Chunk _playerchunk)) _renderdistance) (+ (.Y (Utilities|Struct|BreakS_Chunk _playerchunk)) _renderdistance))
      (if (not (Utilities|Map|Contains (Variables|Default|GetLoadedChunks) (Utilities|Struct|MakeS_Chunk _index _index_2)))
        (if (not (Utilities|Array|ContainsItem _spawnqueue (Utilities|Struct|MakeS_Chunk _index _index_2)))
          (Utilities|Array|Add _spawnqueue (Utilities|Struct|MakeS_Chunk _index _index_2))))))
  (CallFunction|UnloadFarChunks))

(fn GetChunkfromWorld
  (params (X :type Float%20%28double-precision%29) (Y :type Float%20%28double-precision%29) (NewParam :type Rig%20VM%20Function%20Math%20Transform%20Transform%20Vector%20Structure))
  (bind (_chunkblocks _blocksize) (Utilities|GetClassDefaults "/Game/Terrain/DA_TerrainSettings.DA_TerrainSettings_C"))
  (bind _returnvalue (* _chunkblocks _blocksize))
  (return (Utilities|Struct|MakeS_Chunk (Math|Float|Floor (/ X _returnvalue)) (Math|Float|Floor (/ Y _returnvalue)))))

(fn GetfromQueue
  (bind _spawnqueue (Variables|Default|GetSpawnQueue))
  (if (> (Utilities|Array|Length (Variables|Default|GetSpawnQueue)) 0)
    (LocalVariables|SetItem (Utilities|Array|Get(acopy) _spawnqueue))
    (Utilities|Array|RemoveIndex _spawnqueue)
    (return true (LocalVariables|GetItem))
    (else
      (return false ""))))

(fn UnloadFarChunks
  (bind _renderdistance (Variables|Default|GetRenderDistance))
  (bind _loadedchunks (Variables|Default|GetLoadedChunks))
  (bind _returnvalue (+ _renderdistance 1))
  (bind _playerchunk (CallFunction|GetPlayerChunk))
  (bind _keys (Utilities|Map|Keys (Variables|Default|GetLoadedChunks)))
  (bind _array_element (Utilities|Array|ForEachLoopwithBreak _keys)
    (:LoopBody
      (if (or (> (Math|Integer|Absolute(Integer) (- (.X (Utilities|Struct|BreakS_Chunk _array_element)) (.X (Utilities|Struct|BreakS_Chunk _playerchunk)))) _returnvalue) (> (Math|Integer|Absolute(Integer) (- (.Y (Utilities|Struct|BreakS_Chunk _array_element)) (.Y (Utilities|Struct|BreakS_Chunk _playerchunk)))) _returnvalue))
        (if (.ReturnValue (Utilities|Map|Find _loadedchunks _array_element))
          (Actor|DestroyActor (.Value (Utilities|Map|Find _loadedchunks _array_element)))
          (Utilities|Map|Remove _loadedchunks _array_element))))))

(fn GetPlayerChunk
  (bind _returnvalue (Game|Player|GetPlayerPawn 0))
  (bind _returnvalue_2 (Transformation|GetActorLocation _returnvalue))
  (bind (_x _y) (Math|Vector|BreakVector _returnvalue_2))
  (bind _chunk (CallFunction|GetChunkfromWorld _x _y))
  (return _chunk))