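; BP_Chunk is a terrain chunk actor that lays out a flat square grid of tile instances.
; The construction script calls MakeGrid, which adds one Tile instance per block, sized and spaced by Settings.
; CalcWorldPos derives the grid origin from the Chunk X/Y coordinates, shifted by half the chunk width to center it.
; That position is baked into each instance transform, added in the component's local space.
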(event EventBeginPlay)

(fn ConstructionScript
  (CallFunction|MakeGrid))

(fn MakeGrid
  (bind _settings (Variables|Default|GetSettings))
  (bind _settings_2 (Variables|Default|GetSettings))
  (bind _blocksize (Variables|/Game/Terrain/DA_TerrainSettings.DA_TerrainSettings_C|GetBlockSize _settings))
  (bind _chunkblocks (Variables|/Game/Terrain/DA_TerrainSettings.DA_TerrainSettings_C|GetChunkBlocks _settings_2))
  (bind _returnvalue (- _chunkblocks 1))
  (bind _worldposition (CallFunction|CalcWorldPos))
  (LocalVariables|SetWorldPos _worldposition)
  (for _index (range 0 _returnvalue)
    (for _index_2 (range 0 _returnvalue)
      (Components|InstancedStaticMesh|AddInstance (Variables|Default|GetTile) (Math|Transform|MakeTransform (+ (Math|Vector|MakeVector (Math|Conversions|ToFloat(Integer) (* _blocksize _index)) (Math|Conversions|ToFloat(Integer) (* _index_2 _blocksize)) 0.0) (LocalVariables|GetWorldPos))) false))))

(fn CalcCenterOffset
  (bind _settings (Variables|Default|GetSettings))
  (return (* (/ (Math|Conversions|ToFloat(Integer) (Variables|/Game/Terrain/DA_TerrainSettings.DA_TerrainSettings_C|GetChunkBlocks _settings)) 2.0) (Math|Conversions|ToFloat(Integer) (Variables|/Game/Terrain/DA_TerrainSettings.DA_TerrainSettings_C|GetBlockSize _settings)))))

(fn CalcWorldPos
  (bind _chunk (Variables|Default|GetChunk))
  (bind _settings (Variables|Default|GetSettings))
  (bind (_x _y) (Utilities|Struct|BreakS_Chunk _chunk))
  (bind _chunkblocks (Variables|/Game/Terrain/DA_TerrainSettings.DA_TerrainSettings_C|GetChunkBlocks _settings))
  (bind _blocksize (Variables|/Game/Terrain/DA_TerrainSettings.DA_TerrainSettings_C|GetBlockSize _settings))
  (bind _returnvalue (* _chunkblocks _blocksize))
  ;[0.15 0.15 0.15 0.5] Vycentrování chunku
  (bind _center_offset (CallFunction|CalcCenterOffset))
  (return (- (Math|Vector|MakeVector (Math|Conversions|ToFloat(Integer) (* _x _returnvalue)) (Math|Conversions|ToFloat(Integer) (* _returnvalue _y)) 0.0) (Math|Vector|MakeVector _center_offset _center_offset 0.0))))