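; Base character Blueprint that manages health, attacking and a derived idle, moving, attacking or dead state.
; RefreshState picks the state by priority from health, attack flag and velocity, running on a looping timer and after health or attack changes.
; State, HP and death changes fire dispatchers, and death disables movement and capsule collision.
; StartAttack rejects calls while dead or attacking, and a timer scaled by AttackSpeed ends the attack.
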(event Custom|StateTick
  (if (not (Utilities|Enum|Equal(Enum) (Variables|Default|GetState) "NewEnumerator3"))
    (CallFunction|RefreshState)))

(event EventBeginPlay
  (Variables|Default|SetHealth (Variables|Default|GetMaxHealth))
  (Variables|/Script/Engine.CharacterMovementComponent|SetMaxWalkSpeed (Variables|Character|GetCharacterMovement) (Variables|Default|GetWalkSpeed))
  (Utilities|Time|SetTimerbyEvent (delegate Custom|StateTick) 0.1 true true))

(fn ConstructionScript)

(fn RefreshState
  (if (<= (Variables|Default|GetHealth) 0.0)
    (LocalVariables|SetNewState "NewEnumerator3")
    (elif (Variables|Default|GetisAttacking)
      (LocalVariables|SetNewState "NewEnumerator1")
      (elif (Utilities|Operators|NotEqual(!=) :A (Variables|/Script/Engine.MovementComponent|GetVelocity (Variables|Character|GetCharacterMovement)) :ErrorTolerance 3.0)
        (LocalVariables|SetNewState "NewEnumerator4")
        (else
          (LocalVariables|SetNewState "NewEnumerator0")))))
  (if (Utilities|Enum|NotEqual(Enum) (LocalVariables|GetNewState) (Variables|Default|GetState))
    (LocalVariables|SetOldState (Variables|Default|GetState))
    (Variables|Default|SetState (LocalVariables|GetNewState))
    (Default|CallOnStateChange (LocalVariables|GetNewState) (LocalVariables|GetOldState))
    (if (Utilities|Enum|Equal(Enum) (LocalVariables|GetNewState) "NewEnumerator3")
      (Variables|Default|SetisAttacking false)
      (Default|CallOnDeath)
      (Pawn|Components|CharacterMovement|DisableMovement (Variables|Character|GetCharacterMovement))
      (Collision|SetCollisionEnabled (Variables|Collision|GetCapsuleComponent) "NoCollision"))))

(fn SetHP
  (params (NewValue :type Float%20%28double-precision%29))
  (bind _maxhealth (Variables|Default|GetMaxHealth))
  (bind _output_get (Variables|Default|SetHealth (Math|Float|Clamp(Float) NewValue 0.0 _maxhealth)))
  (Default|CallOnHPChanged _output_get _maxhealth)
  (CallFunction|RefreshState))

(fn AnyDamage
  (params (Damage :type Float%20%28double-precision%29))
  (if (Utilities|Enum|NotEqual(Enum) (Variables|Default|GetState) "NewEnumerator3")
    (CallFunction|SetHP (- (Variables|Default|GetHealth) Damage))))

(fn StartAttack
  (bind _state (Variables|Default|GetState))
  (if (or (Utilities|Enum|Equal(Enum) _state "NewEnumerator3") (Utilities|Enum|Equal(Enum) _state "NewEnumerator1"))
    (return false)
    (else
      (Variables|Default|SetisAttacking true)
      (CallFunction|RefreshState)
      (Utilities|Time|SetTimerbyFunctionName 0 "EndAttack" (/ 1.0 (Math|Float|Max(Float) (Variables|Default|GetAttackSpeed) 0.01)))
      (return true))))

(fn EndAttack
  (Variables|Default|SetisAttacking false)
  (CallFunction|RefreshState))